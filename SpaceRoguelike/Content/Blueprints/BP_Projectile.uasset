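; BP_Projectile is the player's weapon projectile, a flipbook fireball that configures itself from the player's equipped weapon.
; On BeginPlay it reads WeaponEquip from player 0 and uses Select nodes to set tint, flipbook, scale and movement speed.
; It also writes that weapon's damage and cooldown back onto BP_Player rather than storing them itself.
; Box overlaps destroy it for any actor except BP_Enemy, whose hits are not handled here.
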(event OnComponentBeginOverlap(Box)
  (params (OverlappedComponent :type Primitive%20Component%20Object%20Reference) (OtherActor :type Actor%20Object%20Reference) (OtherComp :type Primitive%20Component%20Object%20Reference) (OtherBodyIndex :type Integer) (bFromSweep :type Boolean) (SweepResult :type Hit%20Result%20Structure%20%28by%20ref%29))
  (Utilities|Casting|CastToBP_Enemy OtherActor
    (:CastFailed
      (Actor|DestroyActor))))

(event EventBeginPlay
  (bind _paperflipbook (Variables|Default|GetPaperFlipbook))
  (bind _projectilemovement (Variables|Default|GetProjectileMovement))
  (bind _asbp_player (Utilities|Casting|CastToBP_Player (Game|GetPlayerCharacter 0)))
  (bind _output_get (Variables|Default|SetBP_Player _asbp_player))
  (Sprite|SetSpriteColor _paperflipbook (Utilities|Select :Index (Variables|/Game/Blueprints/BP_Player.BP_Player_C|GetWeaponEquip _output_get) :NewEnumerator0 "(R=1.000000,G=1.000000,B=1.000000,A=1.000000)" :NewEnumerator1 "(R=1.000000,G=1.000000,B=1.000000,A=1.000000)" :NewEnumerator2 "(R=0.000000,G=1.000000,B=0.952941,A=1.000000)" :NewEnumerator3 "(R=0.074510,G=1.000000,B=0.000000,A=1.000000)" :NewEnumerator4 "(R=0.650980,G=0.000000,B=1.000000,A=1.000000)"))
  (Sprite|SetFlipbook _paperflipbook (Utilities|Select :Index (Variables|/Game/Blueprints/BP_Player.BP_Player_C|GetWeaponEquip _output_get) :NewEnumerator0 "/Game/Animations/FP_FireBall.FP_FireBall" :NewEnumerator1 "/Game/Animations/FP_FireBall.FP_FireBall" :NewEnumerator2 "/Game/Animations/FP_FireBall.FP_FireBall" :NewEnumerator3 "/Game/Animations/FP_FireBall.FP_FireBall" :NewEnumerator4 "/Game/Animations/FP_FireBall.FP_FireBall"))
  (Transformation|SetActorScale3D (Utilities|Select :Index (Variables|/Game/Blueprints/BP_Player.BP_Player_C|GetWeaponEquip _output_get) :NewEnumerator0 "0.500000,0.500000,0.500000" :NewEnumerator1 "1.000000,0.500000,1.000000" :NewEnumerator2 "0.300000,0.500000,0.300000" :NewEnumerator3 "0.800000,0.500000,0.800000" :NewEnumerator4 "0.600000,0.500000,0.600000"))
  (bind _output_get_2 (Variables|/Script/Engine.ProjectileMovementComponent|SetInitialSpeed _projectilemovement (Utilities|Select :Index (Variables|/Game/Blueprints/BP_Player.BP_Player_C|GetWeaponEquip _output_get) :NewEnumerator0 1e+03 :NewEnumerator1 5e+02 :NewEnumerator2 5e+02 :NewEnumerator3 4e+02 :NewEnumerator4 8e+02)))
  (Variables|/Script/Engine.ProjectileMovementComponent|SetMaxSpeed _projectilemovement _output_get_2)
  (Variables|/Game/Blueprints/BP_Player.BP_Player_C|SetDamageProjectile (Variables|Default|GetBP_Player) (Utilities|Select :Index (Variables|/Game/Blueprints/BP_Player.BP_Player_C|GetWeaponEquip _output_get) :NewEnumerator0 15.0 :NewEnumerator1 25.0 :NewEnumerator2 0.3 :NewEnumerator3 2e+01 :NewEnumerator4 2e+01))
  (Variables|/Game/Blueprints/BP_Player.BP_Player_C|SetCooldownProjectile (Variables|Default|GetBP_Player) (Utilities|Select :Index (Variables|/Game/Blueprints/BP_Player.BP_Player_C|GetWeaponEquip _output_get) :NewEnumerator0 0.4 :NewEnumerator1 0.8 :NewEnumerator2 0.01 :NewEnumerator3 0.5 :NewEnumerator4 0.6)))

(fn ConstructionScript)