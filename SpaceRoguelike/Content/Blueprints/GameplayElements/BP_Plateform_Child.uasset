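; Child platform Blueprint that acts as an elevator, triggered when the player enters BoxElevator.
; BeginPlay positions the top and bottom markers from local offsets and caches their world locations as endpoints.
; On overlap it registers itself as the player's ActorInterract and restarts the Elevator timeline, which lerps Box and Cube between those endpoints.
; End overlap does nothing, and the PlateformStart toggle and debug print are unwired.
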(event OnComponentBeginOverlap(BoxElevator)
  (params (OverlappedComponent :type Primitive%20Component%20Object%20Reference) (OtherActor :type Actor%20Object%20Reference) (OtherComp :type Primitive%20Component%20Object%20Reference) (OtherBodyIndex :type Integer) (bFromSweep :type Boolean) (SweepResult :type Hit%20Result%20Structure%20%28by%20ref%29))
  (bind _asbp_player (Utilities|Casting|CastToBP_Player OtherActor))
  (Variables|/Game/Blueprints/BP_Player.BP_Player_C|SetActorInterract _asbp_player self)
  (bind _move (Timeline|Elevator PlayFromStart)
    (:Update
      (Transformation|SetWorldLocation (Variables|Default|GetBox) (Math|Vector|Lerp(Vector) (Variables|Default|GetElevatorWorldStart) (Variables|Default|GetElevatorWorldEnd) _move) false false))))

(event OnComponentEndOverlap(BoxElevator)
  (params (OverlappedComponent :type Primitive%20Component%20Object%20Reference) (OtherActor :type Actor%20Object%20Reference) (OtherComp :type Primitive%20Component%20Object%20Reference) (OtherBodyIndex :type Integer))
  (Utilities|Casting|CastToBP_Player OtherActor))

(event EventBeginPlay
  (bind _elevatortop (Variables|Default|GetElevatorTop))
  (bind _elevatorbottom (Variables|Default|GetElevatorBottom))
  (|CallParentFunction)
  (Transformation|SetRelativeLocation _elevatortop (Variables|Default|GetElevatorLocalEnd) false false)
  (Variables|Default|SetElevatorWorldEnd (Transformation|GetWorldLocation _elevatortop))
  (Transformation|SetRelativeLocation _elevatorbottom (Variables|Default|GetElevatorLocalStart) false false)
  (Variables|Default|SetElevatorWorldStart (Transformation|GetWorldLocation _elevatorbottom)))

(event EventTick
  (params (DeltaSeconds :type Float%20%28single-precision%29)))

(fn ConstructionScript
  (|CallParentFunction))