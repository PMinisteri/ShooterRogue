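; BP_WeaponPickUp is a world weapon pickup whose type is set by a weapon enum, shown as a tinted Paper2D sprite with a text label.
; The construction script sets sprite, color and label from the enum, while the RandomWeapon event reapplies them with placeholder gun sprites and a new scale.
; Overlapping InterCollision registers the pickup on BP_Player and shows the label; leaving clears the player's pickup flag and hides it.
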(event OnComponentBeginOverlap(InterCollision)
  (params (OverlappedComponent :type Primitive%20Component%20Object%20Reference) (OtherActor :type Actor%20Object%20Reference) (OtherComp :type Primitive%20Component%20Object%20Reference) (OtherBodyIndex :type Integer) (bFromSweep :type Boolean) (SweepResult :type Hit%20Result%20Structure%20%28by%20ref%29))
  (bind _asbp_player (Utilities|Casting|CastToBP_Player OtherActor))
  (bind _output_get (Variables|Default|SetBP_Player _asbp_player))
  (Variables|/Game/Blueprints/BP_Player.BP_Player_C|SetWeaponCanPickUp _output_get self)
  (Variables|/Game/Blueprints/BP_Player.BP_Player_C|SetWeaponPickUp _output_get true)
  (Rendering|SetVisibility (Variables|Default|GetTextRender) true false))

(event OnComponentEndOverlap(InterCollision)
  (params (OverlappedComponent :type Primitive%20Component%20Object%20Reference) (OtherActor :type Actor%20Object%20Reference) (OtherComp :type Primitive%20Component%20Object%20Reference) (OtherBodyIndex :type Integer))
  (bind _asbp_player (Utilities|Casting|CastToBP_Player OtherActor))
  (Variables|/Game/Blueprints/BP_Player.BP_Player_C|SetWeaponPickUp _asbp_player false)
  (Rendering|SetVisibility (Variables|Default|GetTextRender) false false))

(event Custom|RandomWeapon
  (bind _papersprite (Variables|Default|GetPaperSprite))
  (bind _weaponenum (Variables|Default|GetWeaponEnum))
  (Rendering|Components|Sprite|SetSprite _papersprite (Utilities|Select :Index _weaponenum :NewEnumerator0 "/Game/Art/Placeolder_Gun/Placeolder_Gun_PlaceolderSprite_Gun_12.Placeolder_Gun_PlaceolderSprite_Gun_12" :NewEnumerator1 "/Game/Art/Placeolder_Gun/Placeolder_Gun_PlaceolderSprite_Gun_3.Placeolder_Gun_PlaceolderSprite_Gun_3" :NewEnumerator2 "/Game/Art/Placeolder_Gun/Placeolder_Gun_PlaceolderSprite_Gun_2.Placeolder_Gun_PlaceolderSprite_Gun_2" :NewEnumerator3 "/Game/Art/Placeolder_Gun/Placeolder_Gun_PlaceolderSprite_Gun_0.Placeolder_Gun_PlaceolderSprite_Gun_0" :NewEnumerator4 "/Game/Art/Placeolder_Gun/Placeolder_Gun_PlaceolderSprite_Gun_7.Placeolder_Gun_PlaceolderSprite_Gun_7"))
  (Sprite|SetSpriteColor _papersprite (Utilities|Select :Index _weaponenum :NewEnumerator0 "(R=1.000000,G=1.000000,B=1.000000,A=1.000000)" :NewEnumerator1 "(R=1.000000,G=1.000000,B=1.000000,A=1.000000)" :NewEnumerator2 "(R=0.000000,G=1.000000,B=0.952687,A=1.000000)" :NewEnumerator3 "(R=0.077210,G=1.000000,B=0.000000,A=1.000000)" :NewEnumerator4 "(R=0.650980,G=0.000000,B=1.000000,A=1.000000)"))
  (Transformation|SetWorldScale3D _papersprite "0.300000,0.100000,0.300000")
  (Rendering|Components|TextRender|SetText (Variables|Default|GetTextRender) (Utilities|Text|ToText(String) (Utilities|String|EnumtoString _weaponenum))))

(fn ConstructionScript
  (bind _papersprite (Variables|Default|GetPaperSprite))
  (bind _weaponenum (Variables|Default|GetWeaponEnum))
  (Rendering|Components|Sprite|SetSprite _papersprite (Utilities|Select :Index _weaponenum :NewEnumerator0 "/Game/Art/Placeolder_Tiles/32-32A_Sprite.32-32A_Sprite" :NewEnumerator1 "/Game/Art/Placeolder_Tiles/32-32B_Sprite.32-32B_Sprite" :NewEnumerator2 "/Game/Art/Placeolder_Tiles/32-32A_Sprite.32-32A_Sprite" :NewEnumerator3 "/Game/Art/Placeolder_Tiles/32-32A_Sprite.32-32A_Sprite" :NewEnumerator4 "/Game/Art/Placeolder_Tiles/32-32A_Sprite.32-32A_Sprite"))
  (Sprite|SetSpriteColor _papersprite (Utilities|Select :Index _weaponenum :NewEnumerator0 "(R=1.000000,G=1.000000,B=1.000000,A=1.000000)" :NewEnumerator1 "(R=1.000000,G=1.000000,B=1.000000,A=1.000000)" :NewEnumerator2 "(R=0.000000,G=1.000000,B=0.952687,A=1.000000)" :NewEnumerator3 "(R=0.077210,G=1.000000,B=0.000000,A=1.000000)" :NewEnumerator4 "(R=0.650980,G=0.000000,B=1.000000,A=1.000000)"))
  (Rendering|Components|TextRender|SetText (Variables|Default|GetTextRender) (Utilities|Text|ToText(String) (Utilities|String|EnumtoString _weaponenum))))