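; BP_Jumper is a charge-up jump pad that launches BP_Player with a boosted jump after standing in its Box trigger.
; Delay loops count TimerCurrent up each second during overlap and back down after exit; at TimerActivateJump it briefly multiplies JumpZVelocity by ForceJumper, calls Jump, then resets.
; Tick, throttled by a Delay, tints the material by charge progress.
; BeginPlay keeps either the cube or Paper sprite based on the 3D flag.
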(event OnComponentBeginOverlap(Box)
  (params (OverlappedComponent :type Primitive%20Component%20Object%20Reference) (OtherActor :type Actor%20Object%20Reference) (OtherComp :type Primitive%20Component%20Object%20Reference) (OtherBodyIndex :type Integer) (bFromSweep :type Boolean) (SweepResult :type Hit%20Result%20Structure%20%28by%20ref%29))
  (bind _asbp_player (Utilities|Casting|CastToBP_Player OtherActor))
  (Variables|Default|SetBP_Player _asbp_player)
  (bind _output_get (Variables|Default|SetPlayerCanJump true))
  (if _output_get :!label _label
    (Utilities|FlowControl|Delay 1.0)
    (if _output_get
      (if (== (Variables|Default|GetTimerCurrent) (Variables|Default|GetTimerActivateJump))
        (CallFunction|Jumper)
        (goto _label)
        (else
          (bind _result (Math|Float|IncrementFloat (Variables|Default|GetTimerCurrent))
            (:%20%20
              (Variables|Default|SetTimerCurrent _result)
              (goto _label))))))))

(event OnComponentEndOverlap(Box)
  (params (OverlappedComponent :type Primitive%20Component%20Object%20Reference) (OtherActor :type Actor%20Object%20Reference) (OtherComp :type Primitive%20Component%20Object%20Reference) (OtherBodyIndex :type Integer))
  (Utilities|Casting|CastToBP_Player OtherActor)
  (bind _output_get (Variables|Default|SetPlayerCanJump false))
  (if (not _output_get) :!label _label
    (Utilities|FlowControl|Delay 1.0)
    (if (not _output_get)
      (if (> (Variables|Default|GetTimerCurrent) 0.0)
        (bind _result (Math|Float|DecrementFloat (Variables|Default|GetTimerCurrent))
          (:%20%20
            (Variables|Default|SetTimerCurrent _result)
            (goto _label)))
        (else
          (Variables|Default|SetTimerCurrent 0.0))))))

(event Custom|Jumper
  (bind _bp_player (Variables|Default|GetBP_Player)
    (:then
      (bind _output_get (Variables|Default|SetPlayerJumpZVelocity (Variables|/Script/Engine.CharacterMovementComponent|GetJumpZVelocity (Variables|/Script/Engine.Character|GetCharacterMovement _bp_player))))
      (Variables|/Script/Engine.CharacterMovementComponent|SetJumpZVelocity (Variables|/Script/Engine.Character|GetCharacterMovement _bp_player) (* _output_get (Variables|Default|GetForceJumper)))
      (Character|Jump (Variables|Default|GetBP_Player))
      (Utilities|FlowControl|Delay 0.2)
      (Variables|/Script/Engine.CharacterMovementComponent|SetJumpZVelocity (Variables|/Script/Engine.Character|GetCharacterMovement _bp_player) (Variables|Default|GetPlayerJumpZVelocity))
      (Variables|Default|SetTimerCurrent 0.0))
    (:else)))

(event EventTick
  (params (DeltaSeconds :type Float%20%28single-precision%29))
  (bind _timercurrent (Variables|Default|GetTimerCurrent))
  (bind _timeractivatejump (Variables|Default|GetTimerActivateJump))
  (bind _returnvalue (/ _timercurrent _timeractivatejump))
  (bind _returnvalue_2 (- 1.0 _returnvalue))
  (bind _returnvalue_3 (Math|Vector|MakeVector _returnvalue_2 1.0 1.0))
  (Utilities|FlowControl|Delay 1.0)
  (if (Variables|Default|Get3D)
    (Rendering|Material|SetVectorParameterValueonMaterials (Variables|Default|GetCube) "BaseColor" _returnvalue_3)
    (else
      (Rendering|Material|SetVectorParameterValueonMaterials (Variables|Default|GetPaperSprite) "BaseColor" _returnvalue_3))))

(event EventBeginPlay
  (if (Variables|Default|Get3D)
    (Components|DestroyComponent (Variables|Default|GetPaperSprite))
    (else
      (Components|DestroyComponent (Variables|Default|GetCube)))))

(fn ConstructionScript)