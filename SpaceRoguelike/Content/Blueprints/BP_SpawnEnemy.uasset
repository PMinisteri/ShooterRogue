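; Enemy spawner that creates a BP_Enemy of a set type at its PaperSprite location after a delay.
; A player entering the linked TriggerActiveSpawn starts the first spawn once, while a player overlapping the sprite disables spawning.
; Tick uses a DoOnce, reset while the enemy is valid, to request one respawn when it becomes invalid, until the maximum spawn count is reached.
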(event OnComponentBeginOverlap(PaperSprite)
  (params (OverlappedComponent :type Primitive%20Component%20Object%20Reference) (OtherActor :type Actor%20Object%20Reference) (OtherComp :type Primitive%20Component%20Object%20Reference) (OtherBodyIndex :type Integer) (bFromSweep :type Boolean) (SweepResult :type Hit%20Result%20Structure%20%28by%20ref%29))
  (Utilities|Casting|CastToBP_Player OtherActor)
  (Variables|Default|SetEnemyCanSpawn false))

(event OnComponentEndOverlap(PaperSprite)
  (params (OverlappedComponent :type Primitive%20Component%20Object%20Reference) (OtherActor :type Actor%20Object%20Reference) (OtherComp :type Primitive%20Component%20Object%20Reference) (OtherBodyIndex :type Integer))
  (Utilities|Casting|CastToBP_Player OtherActor)
  (Variables|Default|SetEnemyCanSpawn true))

(event OnActorBeginOverlap(TriggerActiveSpawn)
  (params (OverlappedActor :type Actor%20Object%20Reference) (OtherActor :type Actor%20Object%20Reference))
  (Utilities|Casting|CastToBP_Player OtherActor)
  (Utilities|FlowControl|DoOnce false
    (:Completed
      (CallFunction|SpawnEnemy))))

(event Custom|SpawnEnemy
  (bind _papersprite (Variables|Default|GetPaperSprite))
  (bind _returnvalue (Transformation|GetWorldLocation _papersprite))
  (if (Variables|Default|GetEnemyCanSpawn)
    (Utilities|FlowControl|Delay (Variables|Default|GetDelayRespawn))
    (bind _returnvalue_2 (Game|SpawnActorfromClass "/Game/Blueprints/BP_Enemy.BP_Enemy_C" (Math|Transform|MakeTransform (Math|Vector|MakeVector (.x _returnvalue) (+ (.y _returnvalue) 5.0) (.z _returnvalue)) "0, 0, 0" "1,1,1") "Undefined" 0 0))
    (bind _output_get (Variables|Default|SetBP_Enemy _returnvalue_2))
    (Default|SetEnemySpawn _output_get (Variables|Default|GetEnemyType))
    (Variables|Default|SetFirstSpawn false)
    (bind _result (Math|Integer|IncrementInt (Variables|Default|GetNumberEnemySpawnCurrent))
      (:%20%20
        (Variables|Default|SetNumberEnemySpawnCurrent _result)
        (Development|PrintString "Hello")))))

(event EventBeginPlay)

(event EventTick
  (params (DeltaSeconds :type Float%20%28single-precision%29))
  (if (not (Variables|Default|GetFirstSpawn))
    (if (< (Variables|Default|GetNumberEnemySpawnCurrent) (Variables|Default|GetNumberEnemySpawnMax))
      (Variables|Default|GetBP_Enemy
        (:then
          (goto _label Reset))
        (:else
          (Utilities|FlowControl|DoOnce false :!label _label
            (:Completed
              (CallFunction|SpawnEnemy))))))))

(fn ConstructionScript)