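; Side-scrolling follow camera actor that becomes the player's view target and tracks ActorToFollow on X and Z.
; The construction script snaps it to the target; Tick eases the Camera component there with MoveComponentTo at a height offset, faster while BP_Player falls.
; Tick also moves a minimap icon with the player and flips it by facing direction.
; An older dead-zone follow using GetNewXValue and GetNewZValue remains but is disconnected.
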(event EventBeginPlay
  ;[1 1 1] Event Begin Play
  (Game|Player|SetViewTargetwithBlend (Game|GetPlayerController 0) self 0.0 "VTBlend_Linear" 0.0 false)
  (bind _asbp_player (Utilities|Casting|CastToBP_Player (Variables|Default|GetActorToFollow)))
  (Variables|Default|SetBP_Player _asbp_player))

(event EventTick
  (params (DeltaSeconds :type Float%20%28single-precision%29))
  (bind _minimap_icone (Variables|Default|GetMiniMap_Icone))
  (bind _actortofollow (Variables|Default|GetActorToFollow))
  (bind _bp_player (Variables|Default|GetBP_Player))
  (bind _camera (Variables|Default|GetCamera))
  (bind _returnvalue (Transformation|GetActorLocation _bp_player))
  (bind _returnvalue_2 (Transformation|GetActorLocation _actortofollow))
  (bind _returnvalue_3 (Transformation|GetWorldTransform _camera))
  ;[1 1 1] Setup Camera Smooth depending State
  (Utilities|FlowControl|Sequence
    (:then_0
      (if (Variables|/Game/Blueprints/BP_Player.BP_Player_C|GetIsFalling (Variables|Default|GetBP_Player))
        (Variables|Default|SetZlocationState 0.0)
        (Variables|Default|SetOverTime 0.3)
        (else
          (Variables|Default|SetZlocationState 7e+01)
          (Variables|Default|SetOverTime 2.0)))
      (Components|MoveComponentTo _camera (Math|Vector|MakeVector (.x _returnvalue_2) (.y (.location _returnvalue_3)) (+ (.z _returnvalue_2) 42.0)) (.rotation _returnvalue_3) true false (Variables|Default|GetOverTime) false :!label _label)
      (Utilities|FlowControl|Delay 0.0)
      (goto _label Return))
    (:then_1
      ;[1 1 1] IconeMinimap Follow Player
      (Transformation|SetWorldLocation (Variables|Default|GetMiniMap_Icone) (Math|Vector|MakeVector (.x _returnvalue) 5e+01 (.z _returnvalue)) false false)
      ;[1 1 1] IconeRotation Depending Move Player
      (if (Variables|/Game/Blueprints/BP_Player.BP_Player_C|GetMoveRight (Variables|Default|GetBP_Player))
        (Transformation|SetWorldRotation _minimap_icone (Math|Rotator|MakeRotator 0.0 0.0 1.8e+02) false false)
        (else
          (Transformation|SetWorldRotation _minimap_icone (Math|Rotator|MakeRotator 0.0 0.0 0.0) false false))))))

(fn ConstructionScript
  (bind _actortofollow (Variables|Default|GetActorToFollow))
  (bind _returnvalue (Transformation|GetActorLocation _actortofollow))
  ;[1 1 1] Camera Focus Player
  (Transformation|SetActorLocation (Math|Vector|MakeVector (.x _returnvalue) (.y (.location (Transformation|GetWorldTransform (Variables|Default|GetCamera)))) (+ (.z _returnvalue) 42.0)) false false))

(fn GetNewXValue
  (bind _actortofollow (Variables|Default|GetActorToFollow))
  (bind _xdeadzone (Variables|Default|GetXDeadZone))
  (bind _actortofollow_2 (Variables|Default|GetActorToFollow))
  (bind _xdeadzone_2 (Variables|Default|GetXDeadZone))
  (bind _returnvalue (Transformation|GetActorLocation _actortofollow))
  (bind _returnvalue_2 (Transformation|GetActorLocation _actortofollow_2))
  (bind _returnvalue_3 (- (.x _returnvalue) _xdeadzone))
  (bind _returnvalue_4 (+ (.x _returnvalue_2) _xdeadzone_2))
  (if (> _returnvalue_3 (.x (Transformation|GetActorLocation)))
    (return _returnvalue_3)
    (elif (< _returnvalue_4 (.x (Transformation|GetActorLocation)))
      (return _returnvalue_4)
      (else
        (return (Variables|Default|GetCameraX))))))

(fn GetNewZValue
  (bind _actortofollow (Variables|Default|GetActorToFollow))
  (bind _zdeadzone (Variables|Default|GetZDeadZone))
  (bind _actortofollow_2 (Variables|Default|GetActorToFollow))
  (bind _zdeadzone_2 (Variables|Default|GetZDeadZone))
  (bind _returnvalue (Transformation|GetActorLocation _actortofollow))
  (bind _returnvalue_2 (Transformation|GetActorLocation _actortofollow_2))
  (bind _returnvalue_3 (- (.z _returnvalue) _zdeadzone))
  (bind _returnvalue_4 (+ (.z _returnvalue_2) _zdeadzone_2))
  (if (> _returnvalue_3 (.z (Transformation|GetActorLocation)))
    (return _returnvalue_3)
    (elif (< _returnvalue_4 (.z (Transformation|GetActorLocation)))
      (return _returnvalue_4)
      (else
        (Variables|Default|SetCameraCenter false)
        (return (Variables|Default|GetCameraZ))))))