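; BP_Plateform is a platform that is solid to pawns only while the player is inside its Box trigger, which suggests a one-way platform.
; The Cube ignores the Pawn channel from BeginPlay, switches to Block when BP_Player begins overlapping the Box, and reverts to Ignore when that overlap ends.
; A PlayerMoveDown event, also used at BeginPlay, sets the Cube to ignore pawns.
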(event OnComponentBeginOverlap(Box)
  (params (OverlappedComponent :type Primitive%20Component%20Object%20Reference) (OtherActor :type Actor%20Object%20Reference) (OtherComp :type Primitive%20Component%20Object%20Reference) (OtherBodyIndex :type Integer) (bFromSweep :type Boolean) (SweepResult :type Hit%20Result%20Structure%20%28by%20ref%29))
  (Utilities|Casting|CastToBP_Player OtherActor)
  (Collision|SetCollisionResponsetoChannel (Variables|Default|GetCube) "ECC_Pawn" "ECR_Block"))

(event OnComponentEndOverlap(Box)
  (params (OverlappedComponent :type Primitive%20Component%20Object%20Reference) (OtherActor :type Actor%20Object%20Reference) (OtherComp :type Primitive%20Component%20Object%20Reference) (OtherBodyIndex :type Integer))
  (Utilities|Casting|CastToBP_Player OtherActor)
  (Collision|SetCollisionResponsetoChannel (Variables|Default|GetCube) "ECC_Pawn" "ECR_Ignore"))

(event Custom|PlayerMoveDown
  (Collision|SetCollisionResponsetoChannel (Variables|Default|GetCube) "ECC_Pawn" "ECR_Ignore"))

(event EventBeginPlay
  (CallFunction|PlayerMoveDown))

(fn ConstructionScript)