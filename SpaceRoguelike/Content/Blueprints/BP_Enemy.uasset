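; BP_Enemy is a Paper2D droid enemy in two variants, with flipbook and max life selected from EnemyList at construction or through SetEnemySpawn.
; Projectiles hitting BoxTrigger are destroyed and subtract the player's projectile damage, animating the widget life bar and turning the sprite according to the player's X position.
; At zero life it destroys itself and, if DropItems is enabled, spawns a weapon pickup of one of three random types.
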(event OnComponentBeginOverlap(BoxTrigger)
  (params (OverlappedComponent :type Primitive%20Component%20Object%20Reference) (OtherActor :type Actor%20Object%20Reference) (OtherComp :type Primitive%20Component%20Object%20Reference) (OtherBodyIndex :type Integer) (bFromSweep :type Boolean) (SweepResult :type Hit%20Result%20Structure%20%28by%20ref%29))
  (bind _paperflipbook (Variables|Default|GetPaperFlipbook))
  (bind _asbp_projectile (Utilities|Casting|CastToBP_Projectile OtherActor))
  (Actor|DestroyActor _asbp_projectile)
  (Variables|Default|SetCurrentLifeAnimation (Variables|Default|GetCurrentLife))
  (Variables|Default|SetCurrentLife (- (Variables|Default|GetCurrentLife) (Variables|/Game/Blueprints/BP_Player.BP_Player_C|GetDamageProjectile (Variables|Default|GetBP_Player))))
  (if (<= (Variables|Default|GetCurrentLife) 0.0)
    (CallFunction|DropItems)
    (Actor|DestroyActor)
    (else
      ;[1 1 1] LifeBar Widget Update
      (Default|DamageAnimation (Variables|Default|GetW_LifeBar) (Variables|Default|GetCurrentLifeAnimation) (Variables|Default|GetMaxLife) (Variables|Default|GetCurrentLife))
      ;[1 1 1] Flip when damaged
      (if (< (.x (Transformation|GetActorLocation (Variables|Default|GetBP_Player))) (.x (Transformation|GetActorLocation)))
        (Transformation|SetRelativeRotation _paperflipbook "0, 0, 0" false false)
        (else
          (Transformation|SetRelativeRotation _paperflipbook "0,180.000000, 0" false false))))))

(event Custom|DropItems
  (if (Variables|Default|GetDropItems?)
    (bind _returnvalue (Game|SpawnActorfromClass "/Game/Blueprints/BP_WeaponPickUp.BP_WeaponPickUp_C" (Math|Transform|MakeTransform (Transformation|GetWorldLocation (Variables|Default|GetDropWeapon)) "0,90.000000, 0" "1,1,1") "Undefined" 0 0))
    (switch int (Math|Random|RandomIntegerinRange 0 2)
      (:0
        (Variables|/Game/Blueprints/BP_WeaponPickUp.BP_WeaponPickUp_C|SetWeaponEnum _returnvalue "NewEnumerator2"))
      (:1
        (Variables|/Game/Blueprints/BP_WeaponPickUp.BP_WeaponPickUp_C|SetWeaponEnum _returnvalue "NewEnumerator3"))
      (:2
        (Variables|/Game/Blueprints/BP_WeaponPickUp.BP_WeaponPickUp_C|SetWeaponEnum _returnvalue "NewEnumerator4")))
    (Default|RandomWeapon _returnvalue)))

(event Custom|SetEnemySpawn
  (params (EnemyList :type Enum_EnemyList%20Enum :default "NewEnumerator0"))
  (Sprite|SetFlipbook (Variables|Default|GetPaperFlipbook) (Utilities|Select :Index EnemyList :NewEnumerator0 "/Game/Art/Characters/Droide_C_V.Droide_C_V" :NewEnumerator1 "/Game/Art/Characters/Droide_D_V.Droide_D_V"))
  (Variables|Default|SetMaxLife (Utilities|Select :Index EnemyList :NewEnumerator0 5e+01 :NewEnumerator1 3e+01))
  (Variables|Default|SetCurrentLife (Variables|Default|GetMaxLife)))

(event EventBeginPlay
  (bind _asbp_player (Utilities|Casting|CastToBP_Player (Game|GetPlayerCharacter 0)))
  (Variables|Default|SetBP_Player _asbp_player)
  (bind _asw_life_bar (Utilities|Casting|CastToW_LifeBar (UserInterface|GetUserWidgetObject (Variables|Default|GetWidget))))
  (Variables|Default|SetW_LifeBar _asw_life_bar))

(event EventTick
  (params (DeltaSeconds :type Float%20%28single-precision%29)))

(fn ConstructionScript
  (bind _enemylist (Variables|Default|GetEnemyList))
  (Sprite|SetFlipbook (Variables|Default|GetPaperFlipbook) (Utilities|Select :Index _enemylist :NewEnumerator0 "/Game/Art/Characters/Droide_C_V.Droide_C_V" :NewEnumerator1 "/Game/Art/Characters/Droide_D_V.Droide_D_V"))
  (bind _output_get (Variables|Default|SetMaxLife (Utilities|Select :Index _enemylist :NewEnumerator0 5e+01 :NewEnumerator1 3e+01)))
  (Variables|Default|SetCurrentLife _output_get))