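; BP_CluePickUp is a clue pickup actor that tells BP_Player when it can be picked up.
; It caches the player character on BeginPlay and uses two collision volumes to drive the player's pickup state.
; Beginning overlap with InterCollision registers this clue on the player and sets ClueCanPickUp.
; Beginning overlap with OuterCollision clears that flag; no end-overlap events are used.
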(event OnComponentBeginOverlap(InterCollision)
  (params (OverlappedComponent :type Primitive%20Component%20Object%20Reference) (OtherActor :type Actor%20Object%20Reference) (OtherComp :type Primitive%20Component%20Object%20Reference) (OtherBodyIndex :type Integer) (bFromSweep :type Boolean) (SweepResult :type Hit%20Result%20Structure%20%28by%20ref%29))
  (bind _asbp_player (Utilities|Casting|CastToBP_Player OtherActor))
  (bind _output_get (Variables|Default|SetBP_Player _asbp_player))
  (Variables|/Game/Blueprints/BP_Player.BP_Player_C|SetCluePickUp _output_get self)
  (Variables|/Game/Blueprints/BP_Player.BP_Player_C|SetClueCanPickUp _output_get true))

(event OnComponentBeginOverlap(OuterCollision)
  (params (OverlappedComponent :type Primitive%20Component%20Object%20Reference) (OtherActor :type Actor%20Object%20Reference) (OtherComp :type Primitive%20Component%20Object%20Reference) (OtherBodyIndex :type Integer) (bFromSweep :type Boolean) (SweepResult :type Hit%20Result%20Structure%20%28by%20ref%29))
  (bind _asbp_player (Utilities|Casting|CastToBP_Player OtherActor))
  (Variables|/Game/Blueprints/BP_Player.BP_Player_C|SetClueCanPickUp _asbp_player false))

(event EventBeginPlay
  (bind _asbp_player (Utilities|Casting|CastToBP_Player (Game|GetPlayerCharacter 0)))
  (Variables|Default|SetBP_Player _asbp_player))

(fn ConstructionScript)