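; BP_HeatMap paints the player's position into a runtime render target as a heat map, apparently for fog of war.
; Every Tick it traces from the player along world Y to its gathering plane and keeps hits on itself.
; Each hit is converted to plane-local space, remapped to normalized coordinates and stamped with a dynamic M_HeatSplat material.
; The render target is cleared only on BeginPlay, not between stamps.
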(event Custom|DrawToRenderTarget
  (params (Location :type Vector) (Strenght :type Float%20%28single-precision%29) (Size :type Float%20%28single-precision%29))
  (bind _mid_heatsplat (Variables|Default|GetMID_HeatSplat))
  (bind _positiongatheringplane (Variables|Default|GetPositionGatheringPlane))
  (bind _returnvalue (Transformation|GetWorldTransform _positiongatheringplane))
  (bind _returnvalue_2 (Math|Transform|InvertTransform _returnvalue))
  (bind _returnvalue_3 (Math|Transform|TransformLocation _returnvalue_2 Location))
  (Rendering|Material|SetScalarParameterValue _mid_heatsplat "Size" Size :!class /Script/Engine.MaterialInstanceDynamic)
  (Rendering|Material|SetScalarParameterValue _mid_heatsplat "Strenght" Strenght :!class /Script/Engine.MaterialInstanceDynamic)
  (Rendering|Material|SetVectorParameterValue _mid_heatsplat "Position" (Utilities|Struct|MakeLinearColor (/ (* (+ (.x _returnvalue_3) 49.0) 1.44) 139.0) (/ (+ (.y _returnvalue_3) 9e+01) 183.0) 0.0 1.0) :!class /Script/Engine.MaterialInstanceDynamic)
  (Rendering|DrawMaterialtoRenderTarget (Variables|Default|GetRenderTargetRunTime) _mid_heatsplat))

(event EventBeginPlay
  (bind _asbp_player (Utilities|Casting|CastToBP_Player (Game|GetPlayerCharacter 0)))
  (Variables|Default|SetBP_Player _asbp_player)
  (Rendering|ClearRenderTarget2D (Variables|Default|GetRenderTargetRunTime)))

(event EventTick
  (params (DeltaSeconds :type Float%20%28single-precision%29))
  (bind _bp_player (Variables|Default|GetBP_Player))
  (bind _returnvalue (Transformation|GetActorLocation _bp_player))
  (bind (_x _y _z) (Math|Vector|BreakVector _returnvalue))
  (Utilities|IsValid _bp_player
    (:Is%20Valid
      (bind _outhits (Class|KismetSystemLibrary|LineTraceMultiforObjects _returnvalue (Math|Vector|MakeVector _x (- (.y (Transformation|GetWorldLocation (Variables|Default|GetPositionGatheringPlane))) -1.0) _z) (Utilities|Array|MakeArray "ObjectTypeQuery1" "ObjectTypeQuery2") false 0 "None" false))
      (for _array_element _outhits
        (if (and (.bBlockingHit (Collision|BreakHitResult _array_element)) (== (.HitActor (Collision|BreakHitResult _array_element)) self))
          (CallFunction|DrawtoRenderTarget (.Location (Collision|BreakHitResult _array_element)) 5.0 0.06))))))

(fn ConstructionScript
  (bind _returnvalue (Rendering|Material|CreateDynamicMaterialInstance "/Game/Blueprints/FogOfWar/M_HeatSplat.M_HeatSplat" "None" :!class /Script/Engine.KismetMaterialLibrary))
  (Variables|Default|SetMID_HeatSplat _returnvalue))